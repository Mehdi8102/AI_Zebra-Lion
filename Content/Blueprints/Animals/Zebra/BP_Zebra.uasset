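; BP_Zebra is a zebra animal actor that carries a world-space widget UI.
; On BeginPlay it casts the widget component's widget to WDB_Zebra and registers itself as that widget's animal owner.
; Each Tick it billboards the widget by turning only its yaw toward the player camera, a per-frame Blueprint update noted for later C++ reimplementation.
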(event `self.ReceiveBeginPlay`
  (bind _aswdb_zebra (cast `/Game/Blueprints/Animals/Zebra/WDB_Zebra` (`WidgetComponent.GetWidget` (`self.ZebraWidget`))))
  (`/Game/Blueprints/Animals/Zebra/WDB_Zebra.SetAnimalOwner` _aswdb_zebra self))

(event `self.ReceiveTick`
  (params (DeltaSeconds :type "Float (single-precision)"))
  (bind (_returnvalue_roll _returnvalue_pitch _returnvalue_yaw) (`KismetMathLibrary.BreakRotator` (`KismetMathLibrary.FindLookAtRotation` (`SceneComponent.K2_GetComponentLocation` (`self.ZebraWidget`)) (`PlayerCameraManager.GetCameraLocation` (`GameplayStatics.GetPlayerCameraManager` 0)))))
  ;[1 1 1] Should not use tick in BPs! reimplement this in c++ later!
  (`SceneComponent.K2_SetWorldRotation` (`self.ZebraWidget`) (`KismetMathLibrary.MakeRotator` 0.0 0.0 _returnvalue_yaw) false false))

(fn `UserConstructionScript`)