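; AI controller for zebras that runs BT_Zebra on possession and registers lions as predators.
; Each perception update checks every updated actor for sight, hearing and damage stimuli through DeterminePerceivedSense, which matches stimulus sense classes.
; Seen or damage-sensed lions are stored on the zebra and in the Predator blackboard key, using a direct BP_Lion cast pending a Predator base class.
; Hearing only prints debug text.
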(event `self.ReceivePossess`
  (params (PossessedPawn :type "Pawn Object Reference"))
  (`self.RunBehaviorTree` "/Game/Blueprints/Animals/Zebra/AI/BT_Zebra.BT_Zebra"))

(event `self.AIPerception.OnPerceptionUpdated`
  (params (UpdatedActors :type "Array of Actor Object Reference (by ref)"))
  (`KismetSystemLibrary.PrintString` "OnPerception updated called on BP_ZebraAIController" false false)
  (for _array_element UpdatedActors
    (`|ExecutionSequence`
      (:`then_0`
        (bind _array_element_2 (`self.DeterminePerceivedSense` _array_element))
        (if (`.bSuccessfullySensed` (break `AIStimulus` _array_element_2))
          (`self.OnSightSense` _array_element)))
      (:`then_1`
        (bind _array_element_3 (`self.DeterminePerceivedSense` _array_element "NewEnumerator1"))
        (if (`.bSuccessfullySensed` (break `AIStimulus` _array_element_3))
          (`self.OnHearingSense` _array_element)))
      (:`then_2`
        (bind _array_element_4 (`self.DeterminePerceivedSense` _array_element "NewEnumerator4"))
        (if (`.bSuccessfullySensed` (break `AIStimulus` _array_element_4))
          (`self.OnDamageSense` _array_element))))))

(fn `DeterminePerceivedSense`
  (params (SensedActor :type "Actor Object Reference") (Sense :type "/Game/Blueprints/Animals/General_AnimalStuff/E_SenseClass Enum" :default "NewEnumerator0"))
  (returns (`Array Element` :type "AIStimulus Structure"))
  (bind _info (`AIPerceptionComponent.GetActorsPerception` (`self.AIPerception`) SensedActor))
  (for _array_element (`.LastSensedStimuli` (break `ActorPerceptionBlueprintInfo` _info))
    (bind _returnvalue (`AIPerceptionSystem.GetSenseClassForStimulus` _array_element))
    (if (== _returnvalue (select `/Game/Blueprints/Animals/General_AnimalStuff/E_SenseClass` Sense :`NewEnumerator0` "/Script/AIModule.AISense_Sight" :`NewEnumerator1` "/Script/AIModule.AISense_Hearing" :`NewEnumerator4` "/Script/AIModule.AISense_Damage" :!type "AISense Class Reference"))
      (return _array_element))))

(fn `OnDamageSense`
  (params (SensedActor :type "Actor Object Reference"))
  ;[1 1 1] Need to create a Predator class and cast to that instead !
  (bind _asbp_lion (cast `/Game/Blueprints/Animals/Lion/BP_Lion` SensedActor))
  (bind _asbp_zebra (cast `/Game/Blueprints/Animals/Zebra/BP_Zebra` (`self.K2_GetPawn`))
    (:`then`
      (bind _output_get (set `Zebra.Predator` _asbp_lion _asbp_zebra))
      (`BlackboardComponent.SetValueAsObject` (`self.Blackboard`) "Predator" _output_get))
    (:`CastFailed`
      (`KismetSystemLibrary.PrintString` "Cast to BP_Zebra Failed(BP_ZepbraAIController::OnSightSense)"))))

(fn `OnHearingSense`
  (params (HeardActor :type "Actor Object Reference"))
  (`KismetSystemLibrary.PrintString` (`KismetSystemLibrary.GetDisplayName` HeardActor))
  (`KismetSystemLibrary.PrintString` " Was Heard"))

(fn `OnSightSense`
  (params (SeenActor :type "Actor Object Reference"))
  ;[1 1 1] Need to create a Predator class and cast to that instead !
  (bind _asbp_lion (cast `/Game/Blueprints/Animals/Lion/BP_Lion` SeenActor))
  (bind _asbp_zebra (cast `/Game/Blueprints/Animals/Zebra/BP_Zebra` (`self.K2_GetPawn`))
    (:`then`
      (bind _output_get (set `Zebra.Predator` _asbp_lion _asbp_zebra))
      (`BlackboardComponent.SetValueAsObject` (`self.Blackboard`) "Predator" _output_get))
    (:`CastFailed`
      (`KismetSystemLibrary.PrintString` "Cast to BP_Zebra Failed(BP_ZepbraAIController::OnSightSense)"))))

(fn `UserConstructionScript`)