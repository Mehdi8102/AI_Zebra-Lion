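; AI controller for the lion that runs its behavior tree on possession and feeds it prey through AI Perception.
; On each perception update, it checks every updated actor's last stimuli for sight and hearing through a shared lookup by sense class.
; A seen zebra is written to the blackboard as Prey.
; Hearing and forgotten targets only print debug messages, and the damage sense has no class mapped.
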(event `self.ReceivePossess`
  (params (PossessedPawn :type "Pawn Object Reference"))
  ;[1 1 1] Assuming We're possessing a lion!
  (`self.RunBehaviorTree` "/Game/Blueprints/Animals/Lion/AI/BT_Lion.BT_Lion"))

(event `self.AIPerception.OnPerceptionUpdated`
  (params (UpdatedActors :type "Array of Actor Object Reference (by ref)"))
  (`KismetSystemLibrary.PrintString` "OnPerception updated called on BP_LionAIController" false false)
  ;[1 1 1] Not the best intutive way to implement sense specific code(could do better).
  (for _array_element UpdatedActors
    (`|ExecutionSequence`
      (:`then_0`
        (bind _aistimuli (`self.DetermineSensePerceived` _array_element))
        (if (`.bSuccessfullySensed` (break `AIStimulus` _aistimuli))
          (`self.OnSightSense` _array_element)))
      (:`then_1`
        (bind _aistimuli_2 (`self.DetermineSensePerceived` _array_element "NewEnumerator1"))
        (if (`.bSuccessfullySensed` (break `AIStimulus` _aistimuli_2))
          (`self.OnHearingSense` _array_element))))))

(event `self.AIPerception.OnTargetPerceptionForgotten`
  (params (Actor :type "Actor Object Reference"))
  (`KismetSystemLibrary.PrintString` "Bitch" false false))

(fn `DetermineSensePerceived`
  (params (SensedActor :type "Actor Object Reference") (Sense :type "/Game/Blueprints/Animals/General_AnimalStuff/E_SenseClass Enum" :default "NewEnumerator0"))
  (returns (AIStimuli :type "AIStimulus Structure"))
  (locals (E_Sense :type "/Game/Blueprints/Animals/General_AnimalStuff/E_SenseClass Enum" :default "NewEnumerator0"))
  (bind _info (`AIPerceptionComponent.GetActorsPerception` (`self.AIPerception`) SensedActor))
  (for _array_element (`.LastSensedStimuli` (break `ActorPerceptionBlueprintInfo` _info))
    (bind _returnvalue (`AIPerceptionSystem.GetSenseClassForStimulus` _array_element))
    (if (== _returnvalue (select `/Game/Blueprints/Animals/General_AnimalStuff/E_SenseClass` Sense :`NewEnumerator0` "/Script/AIModule.AISense_Sight" :`NewEnumerator1` "/Script/AIModule.AISense_Hearing" :!type "AISense Class Reference"))
      (return _array_element))))

(fn `OnHearingSense`
  (params (HeardActor :type "Actor Object Reference"))
  (`KismetSystemLibrary.PrintString` (`KismetSystemLibrary.GetDisplayName` HeardActor))
  (`KismetSystemLibrary.PrintString` " Was Heard"))

(fn `OnSightSense`
  (params (SeenActor :type "Actor Object Reference"))
  (bind _asbp_zebra (cast `/Game/Blueprints/Animals/Zebra/BP_Zebra` SeenActor))
  (`BlackboardComponent.SetValueAsObject` (`AIBlueprintHelperLibrary.GetBlackboard` null) "Prey" _asbp_zebra))

(fn `UserConstructionScript`)